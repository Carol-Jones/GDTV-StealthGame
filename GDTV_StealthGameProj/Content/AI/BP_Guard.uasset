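; Guard character for a stealth-style game that can capture the player or be taken down by them.
; A radius overlap shows a takedown prompt, and Takedown plays a victim montage, flags the AI controller dead, returns an alignment pose and triggers delayed ragdoll.
; Catch plays a montage whose notify sphere-traces ahead and reports capture to the game mode once.
; Modular body meshes follow the main mesh via leader pose.
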(event OnComponentBeginOverlap(TakedownRadius)
  (params (OverlappedComponent :type Primitive%20Component%20Object%20Reference) (OtherActor :type Actor%20Object%20Reference) (OtherComp :type Primitive%20Component%20Object%20Reference) (OtherBodyIndex :type Integer) (bFromSweep :type Boolean) (SweepResult :type Hit%20Result%20Structure%20%28by%20ref%29))
  (if (and (Actor|ActorHasTag OtherActor "Player") (not (Variables|Default|GetisDead)))
    (Rendering|SetVisibility (Variables|Default|GetTakedownPromptWidget) true false)))

(event OnComponentBeginOverlap(CapsuleComponent)
  (params (OverlappedComponent :type Primitive%20Component%20Object%20Reference) (OtherActor :type Actor%20Object%20Reference) (OtherComp :type Primitive%20Component%20Object%20Reference) (OtherBodyIndex :type Integer) (bFromSweep :type Boolean) (SweepResult :type Hit%20Result%20Structure%20%28by%20ref%29)))

(event OnComponentEndOverlap(TakedownRadius)
  (params (OverlappedComponent :type Primitive%20Component%20Object%20Reference) (OtherActor :type Actor%20Object%20Reference) (OtherComp :type Primitive%20Component%20Object%20Reference) (OtherBodyIndex :type Integer))
  (if (Actor|ActorHasTag OtherActor "Player")
    (Rendering|SetVisibility (Variables|Default|GetTakedownPromptWidget) false false)))

(event Custom|TakedownRagdoll
  (Utilities|FlowControl|Delay 1.27)
  (Physics|SetSimulatePhysics (Variables|Character|GetMesh) true)
  (Pawn|Components|CharacterMovement|SetMovementMode (Variables|Character|GetCharacterMovement) "MOVE_None" 0))

(event EventRun
  (Variables|/Script/Engine.CharacterMovementComponent|SetMaxWalkSpeed (Variables|Character|GetCharacterMovement) 5e+02))

(event EventCatch
  (bind _returnvalue (Transformation|GetActorLocation))
  (if (not (Variables|Default|GetIsAttacking))
    (Animation|Montage|PlayMontage (Variables|Character|GetMesh) "/Game/Characters/PlayerCharacter/Catch/Catch_Montage.Catch_Montage"
      (:then
        (Variables|Default|SetIsAttacking true))
      (:OnCompleted
        (Variables|Default|SetIsAttacking false))
      (:OnNotifyBegin
        (bind (_outhit _returnvalue_2) (Collision|SphereTraceForObjects _returnvalue (+ _returnvalue (* (Transformation|GetActorForwardVector) 135.0)) 5.0 (Utilities|Array|MakeArray "ObjectTypeQuery3") false 0 "ForDuration"))
        (if _returnvalue_2
          (if (Actor|ActorHasTag (.HitActor (Collision|BreakHitResult _outhit)) "Player")
            (Utilities|FlowControl|DoOnce false
              (:Completed
                (bind _asgm_base_game_mode (Utilities|Casting|CastToGM_BaseGameMode (Game|GetGameMode)))
                (Default|PlayerCaptured _asgm_base_game_mode)))))))))

(fn ConstructionScript
  (Components|SkinnedMesh|SetLeaderPoseComponent (Variables|Default|GetLegs) (Variables|Character|GetMesh) false false))

(fn Takedown
  (if (Variables|Default|GetCanTakedown)
    (Animation|PlayAnimMontage "/Game/Characters/PlayerCharacter/Takedowns/Takedown_Victim_Montage.Takedown_Victim_Montage" 1.0 "None")
    (Variables|Default|SetisDead true)
    (bind _asbp_ai_guard (Utilities|Casting|CastToBP_AI_Guard (AI|GetAIController self)))
    (Variables|/Game/AI/BP_AI_Guard.BP_AI_Guard_C|SetIsDead _asbp_ai_guard true)
    (CallFunction|TakedownRagdoll)
    (Rendering|SetVisibility (Variables|Default|GetTakedownPromptWidget) false false)
    (return (Transformation|GetWorldLocation (Variables|Default|GetREF)) (Transformation|GetActorRotation) (Variables|Default|GetCanTakedown) 0)))