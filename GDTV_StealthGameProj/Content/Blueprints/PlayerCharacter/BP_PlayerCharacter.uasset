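; Player character for ground play with Enhanced Input movement and look, a toggled crouch, interaction and guard takedowns.
; Crouching lowers walk speed while timelines blend spring arm, capsule and mesh heights, and an upward sphere trace blocks standing under obstacles.
; Interact messages overlapping BPI_Interact actors and queries overlapping BPI_Guard actors for takedowns.
; An allowed takedown plays the attacker montage, sets a Motion Warping target and ignores the guard during movement.
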(event Input|EnhancedActionEvents|EnhancedInputActionIA_Move
  (params (ActionValue :type Vector%202D%20Structure) (ElapsedSeconds :type Float%20%28double-precision%29) (TriggeredSeconds :type Float%20%28double-precision%29) (InputAction :type Input%20Action%20Object%20Reference :default "/Game/Input/IA_Move.IA_Move"))
  (:Triggered
    (Pawn|Input|AddMovementInput (Math|Vector|GetRightVector (Pawn|GetControlRotation :!class /Script/Engine.Pawn)) (.x ActionValue) false)
    (Pawn|Input|AddMovementInput (Math|Vector|GetForwardVector (Pawn|GetControlRotation :!class /Script/Engine.Pawn)) (.y ActionValue) false)))

(event Input|EnhancedActionEvents|EnhancedInputActionIA_Look
  (params (ActionValue :type Vector%202D%20Structure) (ElapsedSeconds :type Float%20%28double-precision%29) (TriggeredSeconds :type Float%20%28double-precision%29) (InputAction :type Input%20Action%20Object%20Reference :default "/Game/Input/IA_Look.IA_Look"))
  (:Triggered
    (Pawn|Input|AddControllerYawInput (.x ActionValue))
    (Pawn|Input|AddControllerPitchInput (* (.y ActionValue) -1.0))))

(event Input|EnhancedActionEvents|EnhancedInputActionIA_Interact
  (params (ActionValue :type Boolean) (ElapsedSeconds :type Float%20%28double-precision%29) (TriggeredSeconds :type Float%20%28double-precision%29) (InputAction :type Input%20Action%20Object%20Reference :default "/Game/Input/IA_Interact.IA_Interact"))
  (:Started
    (Utilities|FlowControl|Sequence
      (:then_0
        (for _array_element (Collision|GetOverlappingActors 0 :!class /Script/Engine.Actor)
          (if (Utilities|DoesObjectImplementInterface _array_element "/Game/Blueprints/BPI_Interact.BPI_Interact_C")
            (Class|BPIInteract|Interact(Message) _array_element))))
      (:then_1
        (for _array_element_2 (Collision|GetOverlappingActors 0 :!class /Script/Engine.Actor)
          (if (Utilities|DoesObjectImplementInterface _array_element_2 "/Game/Blueprints/Enemy/BPI_Guard.BPI_Guard_C")
            (bind (_ref_pose _rotation _cantakedown _guard) (Class|BPIGuard|Takedown(Message) _array_element_2))
            (if _cantakedown
              (Animation|Montage|PlayMontage (Variables|Character|GetMesh) "/Game/Characters/PlayerCharacter/Takedowns/Takedown_Attacker_Montage.Takedown_Attacker_Montage"
                (:then
                  (Class|MotionWarpingComponent|AddorUpdateWarpTarget (Variables|Default|GetMotionWarping) (Utilities|Struct|MakeMotionWarpingTarget "Takedown" _ref_pose _rotation 0 "None" false))
                  (Collision|IgnoreActorwhenMoving (Variables|Character|GetMesh) _guard true))))))))))

(event Input|EnhancedActionEvents|EnhancedInputActionIA_Crouch
  (params (ActionValue :type Boolean) (ElapsedSeconds :type Float%20%28double-precision%29) (TriggeredSeconds :type Float%20%28double-precision%29) (InputAction :type Input%20Action%20Object%20Reference :default "/Game/Input/IA_Crouch.IA_Crouch"))
  (bind _charactermovement (Variables|Character|GetCharacterMovement))
  (:Started
    (if (not (Variables|Default|GetCrouched))
      (Variables|Default|SetCrouched true)
      (Variables|/Script/Engine.CharacterMovementComponent|SetMaxWalkSpeed _charactermovement 3.5e+02)
      (Utilities|FlowControl|Sequence
        (:then_0
          (bind _zoomspeed (Timeline|CrouchCameraTimeline Play)
            (:Update
              (Transformation|SetRelativeLocation (Variables|Default|GetSpringArm) (Math|Vector|MakeVector 0.0 0.0 (Math|Float|Lerp 7e+01 4e+01 _zoomspeed)) false false))))
        (:then_1
          (bind _capsuleheight (Timeline|CapsuleHeightTimeline Play)
            (:Update
              (Components|Capsule|SetCapsuleHalfHeight (Variables|Collision|GetCapsuleComponent) (Math|Float|Lerp 88.0 5e+01 _capsuleheight) true)
              (Transformation|SetRelativeLocation (Variables|Character|GetMesh) (Math|Vector|MakeVector 0.0 0.0 (Math|Float|Lerp -89.0 -59.0 _capsuleheight)) false false)))))
      (else
        (bind _hit (CallFunction|UncrouchObstableDetection))
        (if (not _hit)
          (Variables|Default|SetCrouched false)
          (Variables|/Script/Engine.CharacterMovementComponent|SetMaxWalkSpeed _charactermovement 6e+02)
          (Utilities|FlowControl|Sequence
            (:then_0
              (Timeline|CrouchCameraTimeline Reverse))
            (:then_1
              (Timeline|CapsuleHeightTimeline Reverse))))))))

(event EventBeginPlay
  (Input|AddMappingContext (PlayerController|LocalPlayerSubsystems|GetEnhancedInputLocalPlayerSubsystem (Game|GetPlayerController 0)) "/Game/Input/IMC_PlayerGround.IMC_PlayerGround" 0 "(bIgnoreAllPressedKeysUntilRelease=True,bForceImmediately=False)"))

(fn ConstructionScript)

(fn UncrouchObstableDetection
  (bind _returnvalue (Transformation|GetActorLocation))
  (bind _returnvalue_2 (Collision|SphereTraceByChannel _returnvalue (+ _returnvalue (* (Math|Vector|GetUpVector (Transformation|GetActorRotation)) 115.0)) 15.0 "TraceTypeQuery1" false 0 "ForDuration"))
  (return _returnvalue_2))