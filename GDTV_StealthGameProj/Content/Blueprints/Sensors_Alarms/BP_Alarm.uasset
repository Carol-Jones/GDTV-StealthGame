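; BP_Alarm is an alarm actor that plays and stops an alarm sound at its own location.
; StartAlarm spawns MS_AlarmSound at the actor's position and keeps the audio component, while StopAlarm fades that sound out linearly.
; An AlarmActive flag guards both events so repeated calls neither stack sounds nor fade an inactive one.
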(event Custom|StartAlarm
  (if (not (Variables|Default|GetAlarmActive))
    (bind _returnvalue (Audio|SpawnSoundatLocation "/Game/Audio/Alarms/MS_AlarmSound.MS_AlarmSound" (Transformation|GetActorLocation) "0, 0, 0" 1.0 1.0 0.0 0 0))
    (Variables|Default|SetAlarmSound _returnvalue)
    (Variables|Default|SetAlarmActive true)))

(event Custom|StopAlarm
  (if (Variables|Default|GetAlarmActive)
    (Audio|Components|Audio|FadeOut (Variables|Default|GetAlarmSound) 1.5 0.0 "Linear" :!class /Script/Engine.AudioComponent)
    (Variables|Default|SetAlarmActive false)))

(fn ConstructionScript)