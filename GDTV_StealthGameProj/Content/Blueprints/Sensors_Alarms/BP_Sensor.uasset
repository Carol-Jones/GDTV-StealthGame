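; BP_Sensor is a detection sensor that triggers the level's alarm when it spots the player.
; Its DetectPlayer event checks the actor's Player tag and fires only once, guarded by a HasDetected flag.
; On detection it plays an attenuated camera shutter sound, starts the alarm on the first BP_Alarm found, and, if one exists, flashes its point light through a timeline.
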(event Custom|DetectPlayer
  (params (ActorDetected :type Actor%20Object%20Reference))
  (if (and (Actor|ActorHasTag ActorDetected "Player") (not (Variables|Default|GetHasDetected)))
    (Variables|Default|SetHasDetected true)
    (Audio|PlaySoundatLocation "/Engine/VREditor/Sounds/UI/Camera_Shutter.Camera_Shutter" (Transformation|GetActorLocation) "0, 0, 0" 1.0 1.0 0.0 "/Game/Audio/Alarms/SA_Sensor.SA_Sensor" 0 0 0)
    (bind _returnvalue (Actor|GetActorOfClass "/Game/Blueprints/Sensors_Alarms/BP_Alarm.BP_Alarm_C"))
    (Utilities|IsValid _returnvalue
      (:Is%20Valid
        (Default|StartAlarm _returnvalue)
        (bind _intensity (Timeline|PointLightFlashTimeline Play)
          (:Update
            (Rendering|Components|Light|SetIntensity (Variables|Default|GetPointLight) (Math|Float|Lerp 0.0 1e+05 _intensity))))))))

(fn ConstructionScript)