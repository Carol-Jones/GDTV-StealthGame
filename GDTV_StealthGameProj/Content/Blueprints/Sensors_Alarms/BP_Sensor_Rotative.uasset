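; Rotating alarm sensor that sweeps its head side to side on a ping-pong timeline and detects the player.
; When the player enters the trigger zone, a series of offset sphere traces along X or Y, chosen by a flag, checks for a hit.
; A hit starts a looping timer that fills the player's detection meter and raises detection when full.
; Leaving the zone drains the meter unless the alert is active.
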(event OnComponentBeginOverlap(TriggerDetectionZone)
  (params (OverlappedComponent :type Primitive%20Component%20Object%20Reference) (OtherActor :type Actor%20Object%20Reference) (OtherComp :type Primitive%20Component%20Object%20Reference) (OtherBodyIndex :type Integer) (bFromSweep :type Boolean) (SweepResult :type Hit%20Result%20Structure%20%28by%20ref%29))
  (if (Actor|ActorHasTag OtherActor "Player")
    (if (Variables|Default|GetShouldLineTraceX)
      (bind _hitplayer (CallFunction|LineTraceX))
      (if _hitplayer
        (Variables|Default|SetPlayerInZone true)
        (bind _returnvalue (Utilities|Time|SetTimerbyEvent (delegate Custom|Count) 0.002 true :!label _label))
        (Variables|Default|SetCountTimer _returnvalue)
        (else
          (Variables|Default|SetPlayerInZone false :!label _label_2)))
      (else
        (bind _didhitplayer (CallFunction|LineTraceY))
        (if _didhitplayer
          (Variables|Default|SetPlayerInZone true)
          (goto _label)
          (else
            (goto _label_2)))))))

(event OnComponentEndOverlap(TriggerDetectionZone)
  (params (OverlappedComponent :type Primitive%20Component%20Object%20Reference) (OtherActor :type Actor%20Object%20Reference) (OtherComp :type Primitive%20Component%20Object%20Reference) (OtherBodyIndex :type Integer))
  (Utilities|Time|ClearandInvalidateTimerbyHandle (Variables|Default|GetCountTimer))
  (if (Actor|ActorHasTag OtherActor "Player")
    (Variables|Default|SetPlayerInZone false)
    (bind _returnvalue (Utilities|Time|SetTimerbyEvent (delegate Custom|Decount) 0.002 true))
    (Variables|Default|SetDecountTimer _returnvalue)))

(event Custom|Count
  (Variables|Default|SetTimeUnderZone (+ (Variables|Default|GetTimeUnderZone) 0.005))
  (CallFunction|UpdateProgressBar)
  (if (>= (Variables|Default|GetTimeUnderZone) 3.0)
    (CallFunction|DetectPlayer (stale OnComponentBeginOverlap(TriggerDetectionZone) OtherActor))
    (Utilities|Time|ClearandInvalidateTimerbyHandle (Variables|Default|GetCountTimer))
    (Default|PlayerDetected (Variables|/Game/Blueprints/PlayerCharacter/BP_PlayerCharacter.BP_PlayerCharacter_C|GetDetectedMeterWidget (Variables|Default|GetPlayerCharacter)))))

(event Custom|UpdateProgressBar
  (if (not (Variables|/Game/UI/WB_AlertMeter.WB_AlertMeter_C|GetAlertStatus (Variables|/Game/Blueprints/PlayerCharacter/BP_PlayerCharacter.BP_PlayerCharacter_C|GetDetectedMeterWidget (Variables|Default|GetPlayerCharacter))))
    (Progress|SetPercent (Variables|/Game/UI/WB_AlertMeter.WB_AlertMeter_C|GetDetectionProgressBar (Variables|/Game/Blueprints/PlayerCharacter/BP_PlayerCharacter.BP_PlayerCharacter_C|GetDetectedMeterWidget (Variables|Default|GetPlayerCharacter))) (/ (Variables|Default|GetTimeUnderZone) 3.0))))

(event Custom|Decount
  (if (not (Variables|/Game/UI/WB_AlertMeter.WB_AlertMeter_C|GetAlertStatus (Variables|/Game/Blueprints/PlayerCharacter/BP_PlayerCharacter.BP_PlayerCharacter_C|GetDetectedMeterWidget (Variables|Default|GetPlayerCharacter))))
    (Variables|Default|SetTimeUnderZone (- (Variables|Default|GetTimeUnderZone) 0.003))
    (CallFunction|UpdateProgressBar)
    (if (<= (Variables|Default|GetTimeUnderZone) 0.0)
      (Utilities|Time|ClearandInvalidateTimerbyHandle (Variables|Default|GetDecountTimer)))))

(event EventBeginPlay
  (bind _head (Variables|Default|GetHead))
  (bind _relativerotation (Variables|/Script/Engine.SceneComponent|GetRelativeRotation _head))
  (Utilities|FlowControl|Sequence
    (:then_0
      (Audio|PlaySoundatLocation "/Game/Audio/Alarms/SensorAmbience.SensorAmbience" (Transformation|GetWorldLocation (Variables|Default|GetDefaultSceneRoot)) "0, 0, 0" 0.2 1.0 0.0 "/Game/Audio/Alarms/SA_Sensor.SA_Sensor" 0 0 0)
      (bind _rotation (Timeline|Motion Play)
        (:Update
          (Transformation|SetRelativeRotation _head (Math|Rotator|Lerp(Rotator) (Math|Rotator|MakeRotator (.roll _relativerotation) (.pitch _relativerotation) 35.0) (Math|Rotator|MakeRotator (.roll _relativerotation) (.pitch _relativerotation) -35.0) _rotation) false false))
        (:Finished
          (Utilities|FlowControl|FlipFlop
            (:A
              (Timeline|Motion Reverse))
            (:B
              (Timeline|Motion Play))))))
    (:then_1
      (bind _asbp_player_character (Utilities|Casting|CastToBP_PlayerCharacter (Game|GetPlayerCharacter 0)))
      (Variables|Default|SetPlayerCharacter _asbp_player_character))))

(fn ConstructionScript
  (|CallParentFunction))

(fn LineTraceY
  (Variables|Default|SetLineTraceShiftAmount -2.0)
  (bind _index (Utilities|FlowControl|ForLoopwithBreak 0 40)
    (:LoopBody
      (Variables|Default|SetLineTraceShiftAmount (+ (Variables|Default|GetLineTraceShiftAmount) (* _index 2)))
      (bind (_outhit _returnvalue) (Collision|SphereTraceByChannel (+ (Transformation|GetWorldLocation (Variables|Default|GetScanLineStart)) (Math|Vector|MakeVector 0.0 (Variables|Default|GetLineTraceShiftAmount) -5e+01)) (+ (Transformation|GetWorldLocation (Variables|Default|GetHead)) (* (Math|Vector|GetForwardVector (Transformation|GetWorldRotation (Variables|Default|GetHead))) 1e+04)) 75.0 "TraceTypeQuery2" true 0 "ForDuration"))
      (if _returnvalue
        (if (Actor|ActorHasTag (.HitActor (Collision|BreakHitResult _outhit)) "Player")
          (Development|PrintString "Player Found")
          (return _returnvalue))))
    (:Completed
      (return _returnvalue))))

(fn LineTraceX
  (Variables|Default|SetLineTraceShiftAmount -2.0)
  (bind _index (Utilities|FlowControl|ForLoopwithBreak 0 40)
    (:LoopBody
      (Variables|Default|SetLineTraceShiftAmount (+ (Variables|Default|GetLineTraceShiftAmount) (* _index 2)))
      (bind (_outhit _returnvalue) (Collision|SphereTraceByChannel (+ (Transformation|GetWorldLocation (Variables|Default|GetScanLineStart)) (Math|Vector|MakeVector (Variables|Default|GetLineTraceShiftAmount) 0.0 -5e+01)) (+ (Transformation|GetWorldLocation (Variables|Default|GetHead)) (* (Math|Vector|GetForwardVector (Transformation|GetWorldRotation (Variables|Default|GetHead))) 1e+04)) 75.0 "TraceTypeQuery2" true 0 "ForDuration"))
      (if _returnvalue
        (if (Actor|ActorHasTag (.HitActor (Collision|BreakHitResult _outhit)) "Player")
          (return _returnvalue))))
    (:Completed
      (return _returnvalue))))