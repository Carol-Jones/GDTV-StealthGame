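; BP_Lever is an interactable wall or world switch that toggles a linked OutputActor.
; Interact calls SwitchLever, which messages the output through BPI_Interact, flips Activated, plays a switch sound and runs the PullLever timeline forward or in reverse to rotate the handle.
; Without a valid output implementing that interface, the lever does nothing.
; A trigger overlap shows or hides a use-prompt widget for Player-tagged actors.
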(event OnComponentBeginOverlap(PromptTrigger)
  (params (OverlappedComponent :type Primitive%20Component%20Object%20Reference) (OtherActor :type Actor%20Object%20Reference) (OtherComp :type Primitive%20Component%20Object%20Reference) (OtherBodyIndex :type Integer) (bFromSweep :type Boolean) (SweepResult :type Hit%20Result%20Structure%20%28by%20ref%29))
  (if (Actor|ActorHasTag OtherActor "Player")
    (bind _aswb_use_prompt (Utilities|Casting|CastToWB_UsePrompt (UserInterface|GetWidget (Variables|Default|GetPromptWidget))))
    (Variables|/Script/UMG.TextBlock|SetText (Variables|/Game/UI/WB_UsePrompt.WB_UsePrompt_C|GetPromptText _aswb_use_prompt) "[E] 
Switch On/Off")
    (Rendering|SetVisibility (Variables|Default|GetPromptWidget) true false)))

(event OnComponentEndOverlap(PromptTrigger)
  (params (OverlappedComponent :type Primitive%20Component%20Object%20Reference) (OtherActor :type Actor%20Object%20Reference) (OtherComp :type Primitive%20Component%20Object%20Reference) (OtherBodyIndex :type Integer))
  (if (Actor|ActorHasTag OtherActor "Player")
    (Rendering|SetVisibility (Variables|Default|GetPromptWidget) false false)))

(event Custom|SwitchLever
  (bind _outputactor (Variables|Default|GetOutputActor)
    (:then
      (if (Utilities|DoesObjectImplementInterface _outputactor "/Game/Blueprints/BPI_Interact.BPI_Interact_C")
        (Class|BPIInteract|Interact(Message) _outputactor)
        (if (not (Variables|Default|GetActivated))
          (Audio|PlaySoundatLocation "/Game/Audio/Switch/switch_off.switch_off" (Transformation|GetWorldLocation (Variables|Default|GetDefaultSceneRoot)) "0, 0, 0" 1.0 1.0 0.0 "/Game/Audio/Alarms/SA_Sensor.SA_Sensor" 0 0 0)
          (Variables|Default|SetActivated true)
          (bind _rotation (Timeline|PullLever Play)
            (:Update
              (Transformation|SetRelativeRotation (Variables|Default|GetLever) (Math|Rotator|Lerp(Rotator) "0.000000,0.000000,-50.000000" "0.000000,0.000000,-120.000000" _rotation) false false)))
          (else
            (Audio|PlaySoundatLocation "/Game/Audio/Switch/switch_on.switch_on" (Transformation|GetWorldLocation (Variables|Default|GetDefaultSceneRoot)) "0, 0, 0" 1.0 1.0 0.0 "/Game/Audio/Alarms/SA_Sensor.SA_Sensor" 0 0 0)
            (Variables|Default|SetActivated false)
            (Timeline|PullLever Reverse)))))
    (:else)))

(event EventInteract
  (CallFunction|SwitchLever))

(fn ConstructionScript)