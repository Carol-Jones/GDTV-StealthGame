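; Interactable hinged door that swings open 90 degrees away from or toward zero yaw and plays open and close sounds.
; Two trigger boxes track which side a Player-tagged actor stands on and show that side's WB_UsePrompt widget with open or close text.
; Interact toggles the open state, hides both prompts and uses the side to sign the yaw, which timelines lerp as relative rotation, independent of placement angle.
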(event OnComponentBeginOverlap(CloseDoorTriggerBox)
  (params (OverlappedComponent :type Primitive%20Component%20Object%20Reference) (OtherActor :type Actor%20Object%20Reference) (OtherComp :type Primitive%20Component%20Object%20Reference) (OtherBodyIndex :type Integer) (bFromSweep :type Boolean) (SweepResult :type Hit%20Result%20Structure%20%28by%20ref%29))
  ;[0 0.07887 1 1 48] Triggerbox Logic for the door to determine when to show prompt and toggle the bool for which side of the door they are on.
  (if (Variables|Default|GetIsOpen)
    (if (Actor|ActorHasTag OtherActor "Player")
      (bind _aswb_use_prompt (Utilities|Casting|CastToWB_UsePrompt (UserInterface|GetWidget (Variables|Default|GetCloseDoorWidget))))
      (Variables|/Script/UMG.TextBlock|SetText (Variables|/Game/UI/WB_UsePrompt.WB_UsePrompt_C|GetPromptText _aswb_use_prompt) "[E] 
Close Door")
      (Rendering|SetVisibility (Variables|Default|GetCloseDoorWidget) true false)
      (Variables|Default|SetIsOnNegativeSide true))
    (elif (Actor|ActorHasTag OtherActor "Player")
      (bind _aswb_use_prompt_2 (Utilities|Casting|CastToWB_UsePrompt (UserInterface|GetWidget (Variables|Default|GetCloseDoorWidget))))
      (Variables|/Script/UMG.TextBlock|SetText (Variables|/Game/UI/WB_UsePrompt.WB_UsePrompt_C|GetPromptText _aswb_use_prompt_2) "[E] 
Open Door")
      (Rendering|SetVisibility (Variables|Default|GetCloseDoorWidget) true false)
      (Variables|Default|SetIsOnNegativeSide true))))

(event OnComponentEndOverlap(CloseDoorTriggerBox)
  (params (OverlappedComponent :type Primitive%20Component%20Object%20Reference) (OtherActor :type Actor%20Object%20Reference) (OtherComp :type Primitive%20Component%20Object%20Reference) (OtherBodyIndex :type Integer))
  ;[0 0.07887 1 1 48] Triggerbox Logic for the door to determine when to show prompt and toggle the bool for which side of the door they are on.
  (if (Actor|ActorHasTag OtherActor "Player")
    (Rendering|SetVisibility (Variables|Default|GetCloseDoorWidget) false false)
    (Variables|Default|SetIsOnNegativeSide false)))

(event OnComponentBeginOverlap(OpenDoorTriggerBox)
  (params (OverlappedComponent :type Primitive%20Component%20Object%20Reference) (OtherActor :type Actor%20Object%20Reference) (OtherComp :type Primitive%20Component%20Object%20Reference) (OtherBodyIndex :type Integer) (bFromSweep :type Boolean) (SweepResult :type Hit%20Result%20Structure%20%28by%20ref%29))
  ;[0 0.07887 1 1 48] Triggerbox Logic for the door to determine when to show prompt and toggle the bool for which side of the door they are on.
  (if (not (Variables|Default|GetIsOpen))
    (if (Actor|ActorHasTag OtherActor "Player")
      (bind _aswb_use_prompt (Utilities|Casting|CastToWB_UsePrompt (UserInterface|GetWidget (Variables|Default|GetOpenDoorWidget))))
      (Variables|/Script/UMG.TextBlock|SetText (Variables|/Game/UI/WB_UsePrompt.WB_UsePrompt_C|GetPromptText _aswb_use_prompt) "[E] 
Open Door")
      (Rendering|SetVisibility (Variables|Default|GetOpenDoorWidget) true false)
      (Variables|Default|SetIsOnPositiveSide true))
    (elif (Actor|ActorHasTag OtherActor "Player")
      (bind _aswb_use_prompt_2 (Utilities|Casting|CastToWB_UsePrompt (UserInterface|GetWidget (Variables|Default|GetOpenDoorWidget))))
      (Variables|/Script/UMG.TextBlock|SetText (Variables|/Game/UI/WB_UsePrompt.WB_UsePrompt_C|GetPromptText _aswb_use_prompt_2) "[E] 
Close Door")
      (Rendering|SetVisibility (Variables|Default|GetOpenDoorWidget) true false)
      (Variables|Default|SetIsOnPositiveSide true))))

(event OnComponentEndOverlap(OpenDoorTriggerBox)
  (params (OverlappedComponent :type Primitive%20Component%20Object%20Reference) (OtherActor :type Actor%20Object%20Reference) (OtherComp :type Primitive%20Component%20Object%20Reference) (OtherBodyIndex :type Integer))
  ;[0 0.07887 1 1 48] Triggerbox Logic for the door to determine when to show prompt and toggle the bool for which side of the door they are on.
  (if (Actor|ActorHasTag OtherActor "Player")
    (Rendering|SetVisibility (Variables|Default|GetOpenDoorWidget) false false)
    (Variables|Default|SetIsOnPositiveSide false)))

(event EventInteract
  (bind _door (Variables|Default|GetDoor))
  (bind _returnvalue (Transformation|GetWorldLocation _door))
  ;[0 0.1138 1 1 48] Interact Event for Door - Checks which side of the door the player is on, uses logic to allow for any angle of placement, door will always open at 90 degrees.
  (if (not (Variables|Default|GetIsOpen))
    (Variables|Default|SetIsOpen true)
    (Audio|PlaySoundatLocation "/Game/Audio/door/Door_Open.Door_Open" _returnvalue "0, 0, 0" 1.0 1.0 0.0 0 0 0 0)
    (Rendering|SetVisibility (Variables|Default|GetOpenDoorWidget) false false)
    (if (Variables|Default|GetIsOnPositiveSide)
      (Variables|Default|SetDoorRotation 9e+01)
      (bind _rotation (Timeline|OpenDoor PlayFromStart)
        (:Update
          (Transformation|SetRelativeRotation (Variables|Default|GetDoor) (Math|Rotator|Lerp(Rotator) (Math|Rotator|MakeRotator 0.0 0.0 0.0) (Math|Rotator|MakeRotator 0.0 0.0 (Variables|Default|GetDoorRotation)) _rotation) false false)))
      (elif (Variables|Default|GetIsOnNegativeSide)
        (Variables|Default|SetDoorRotation -9e+01)
        (Timeline|OpenDoor PlayFromStart)))
    (else
      (Variables|Default|SetIsOpen false)
      (Audio|PlaySoundatLocation "/Game/Audio/door/Door_Close.Door_Close" _returnvalue "0, 0, 0" 1.0 1.0 0.0 0 0 0 0)
      (Rendering|SetVisibility (Variables|Default|GetCloseDoorWidget) false false)
      (if (Variables|Default|GetIsOnPositiveSide)
        (bind _rotation_2 (Timeline|CloseDoor PlayFromStart)
          (:Update
            (Transformation|SetRelativeRotation (Variables|Default|GetDoor) (Math|Rotator|Lerp(Rotator) (Math|Rotator|MakeRotator 0.0 0.0 (Variables|Default|GetDoorRotation)) (Math|Rotator|MakeRotator 0.0 0.0 0.0) _rotation_2) false false)))
        (elif (Variables|Default|GetIsOnNegativeSide)
          (Timeline|CloseDoor PlayFromStart))))))

(fn ConstructionScript)