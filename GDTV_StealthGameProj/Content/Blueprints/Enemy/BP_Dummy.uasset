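; Dummy enemy character that can be the victim of a player-triggered takedown.
; An overlap radius shows a takedown prompt widget to Player-tagged actors while it is alive and hides it when they leave.
; Takedown, gated by CanTakedown, plays the victim montage, marks it dead, hides the prompt and returns a reference location and rotation to the caller.
; After a fixed delay, the mesh switches to ragdoll physics and movement is disabled.
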(event OnComponentBeginOverlap(TakedownRadius)
  (params (OverlappedComponent :type Primitive%20Component%20Object%20Reference) (OtherActor :type Actor%20Object%20Reference) (OtherComp :type Primitive%20Component%20Object%20Reference) (OtherBodyIndex :type Integer) (bFromSweep :type Boolean) (SweepResult :type Hit%20Result%20Structure%20%28by%20ref%29))
  (if (and (Actor|ActorHasTag OtherActor "Player") (not (Variables|Default|GetisDead)))
    (Rendering|SetVisibility (Variables|Default|GetTakedownPromptWidget) true false)))

(event OnComponentEndOverlap(TakedownRadius)
  (params (OverlappedComponent :type Primitive%20Component%20Object%20Reference) (OtherActor :type Actor%20Object%20Reference) (OtherComp :type Primitive%20Component%20Object%20Reference) (OtherBodyIndex :type Integer))
  (if (Actor|ActorHasTag OtherActor "Player")
    (Rendering|SetVisibility (Variables|Default|GetTakedownPromptWidget) false false)))

(event Custom|TakedownRagdoll
  (Utilities|FlowControl|Delay 1.27)
  (Physics|SetSimulatePhysics (Variables|Character|GetMesh) true)
  (Pawn|Components|CharacterMovement|SetMovementMode (Variables|Character|GetCharacterMovement) "MOVE_None" 0))

(fn ConstructionScript)

(fn Takedown
  (if (Variables|Default|GetCanTakedown)
    (Animation|PlayAnimMontage "/Game/Characters/PlayerCharacter/Takedowns/Takedown_Victim_Montage.Takedown_Victim_Montage" 1.0 "None")
    (Variables|Default|SetisDead true)
    (CallFunction|TakedownRagdoll)
    (Rendering|SetVisibility (Variables|Default|GetTakedownPromptWidget) false false)
    (return (Transformation|GetWorldLocation (Variables|Default|GetREF)) (Transformation|GetActorRotation) (Variables|Default|GetCanTakedown) 0)))